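; Gameplay ability that equips the player's crafted sword, activatable only with a valid right-hand inventory weapon.
; Plays the equip montage and, on its gameplay event, attaches the weapon to the hand socket and hands it to the combat component.
; The ability ends with the montage.
; HandleEquipWeapon, uncalled here, links the weapon anim layer and grants abilities on authority, and adds the input mapping context locally.
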(event Ability|EventActivateAbility
  (Development|PrintString "Equip")
  (|PlayMontageandWaitProxy "None" "/Game/Animations/Armot/AM_Warrior_Equip.AM_Warrior_Equip" 1.0 "None" true 1.0 0.0 false
    (:then
      (Ability|Tasks|WaitGameplayEvent "(TagName=\"Player.Event.Equip.Sword\")" 0
        (:then
          (Class|PlayerCombatComponent|GetPlayerCarriedWeaponbyTagSafe (Class|DDSPlayerGameplayAbility|GetPlayerCombatComponentfromActorInfo) "(TagName=\"Player.Weapon.Crafted\")" true))
        (:EventReceived
          (Transformation|AttachComponentToComponent (Class|PlayerCombatComponent|GetPlayerCarriedWeaponbyTag (Class|DDSPlayerGameplayAbility|GetPlayerCombatComponentfromActorInfo) "(TagName=\"Player.Weapon.Crafted\")") (Class|GameplayAbility|GetOwningComponentfromActorInfo) "RightHandSwordSlot" "SnapToTarget" "KeepRelative" "KeepWorld" true)
          (Class|PawnCombatComponent|HandleWeaponEquip (Class|DDSPlayerGameplayAbility|GetPlayerCombatComponentfromActorInfo) (Class|PlayerCombatComponent|GetPlayerCarriedWeaponbyTag (Class|DDSPlayerGameplayAbility|GetPlayerCombatComponentfromActorInfo) "(TagName=\"Player.Weapon.Crafted\")"))
          (Variables|/Script/DDS.PawnCombatComponent|SetCurrentEquippedWeaponTag (Class|DDSPlayerGameplayAbility|GetPlayerCombatComponentfromActorInfo) "(TagName=\"Player.Weapon.Crafted\")"))))
    (:OnCompleted
      (Ability|EndAbility :!label _label))
    (:OnBlendOut
      (goto _label))
    (:OnInterrupted
      (goto _label))
    (:OnCancelled
      (goto _label))))

(event Ability|EventOnEndAbility
  (params (bWasCancelled :type Boolean)))

(fn HandleEquipWeapon
  (params (InWeaponToEquip :type DDS%20Crafted%20Player%20Weapon%20Object%20Reference))
  (Utilities|String|LogString (Utilities|GetDisplayName InWeaponToEquip))
  (LocalVariables|SetChachedPlayerWeaponData (Variables|/Script/DDS.DDSSimplePlayerWeapon|GetPlayerWeaponData InWeaponToEquip))
  (Utilities|FlowControl|Sequence
    (:then_0
      (Ability|HasAuthority
        (:True
          (Class|EntityBase|MulticastLinkAnimLayer (Class|DDSPlayerGameplayAbility|GetPlayerCharacterfromActorInfo) (.WeaponAnimLayerToLink (Utilities|Struct|BreakDDSBaseWeaponData (LocalVariables|GetChachedPlayerWeaponData)))))))
    (:then_1
      (Pawn|IsLocallyControlled
        (:True
          (Input|AddMappingContext (PlayerController|LocalPlayerSubsystems|GetEnhancedInputLocalPlayerSubsystem (Class|DDSPlayerGameplayAbility|GetIngamePlayerControllerfromActorInfo)) (.WeaponInputMappingContext (Utilities|Struct|BreakDDSBaseWeaponData (LocalVariables|GetChachedPlayerWeaponData))) 1 "(bIgnoreAllPressedKeysUntilRelease=True,bForceImmediately=False,bNotifyUserSettings=False)"))))
    (:then_2
      (Ability|HasAuthority
        (:True
          (bind _outhandles (Class|DDSAbilitySystemComponent|GrantPlayerWeaponAbilities (Class|DDSGameplayAbility|GetDDSAbilitySystemComponentfromActorInfo) (.DefaultWeaponAbilities (Utilities|Struct|BreakDDSBaseWeaponData (LocalVariables|GetChachedPlayerWeaponData))) (Ability|GetAbilityLevel)))
          (Class|DDSWeaponBase|AssignGrantedAbilitySpecHandles InWeaponToEquip _outhandles))))))

(fn K2CanActivateAbility
  (params (ActorInfo :type Gameplay%20Ability%20Actor%20Info%20Structure) (Handle :type Gameplay%20Ability%20Spec%20Handle%20Structure))
  (bind _asbp_tplayer (Utilities|Casting|CastToBP_TPlayer (.AvatarActor (Utilities|Struct|BreakGameplayAbilityActorInfo ActorInfo))))
  (bind _returnvalue (Class|PlayerBase|GetInventoryComponent _asbp_tplayer))
  (Development|PrintString (Utilities|String|ToString(Boolean) (Utilities|IsValid (Class|InventoryComponent|GetRightWeaponItem _returnvalue))))
  (return "" (Utilities|IsValid (Class|InventoryComponent|GetRightWeaponItem _returnvalue))))