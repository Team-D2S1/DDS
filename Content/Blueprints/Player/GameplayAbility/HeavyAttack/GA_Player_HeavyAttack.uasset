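; Player heavy attack gameplay ability that steps through a combo of montages, one per activation.
; Activation clears the pending reset timer, plays the montage mapped to the combo count, then advances the count, wrapping after the last entry.
; Any montage exit ends the ability and starts a short timer that resets the combo.
; The counter is named as a light attack count despite serving the heavy attack.
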(event Custom|ResetAttackComboCount
  (Variables|Default|SetCurrentLgihtAttackComboCount 1))

(event Ability|EventActivateAbility
  (Utilities|Time|ClearandInvalidateTimerbyHandle (Variables|Default|GetComboCountResetTimerHandle))
  (|PlayMontageandWaitProxy "None" (.Value (Utilities|Map|Find (Variables|Default|GetAttackMontageMap) (Variables|Default|GetCurrentLgihtAttackComboCount))) 1.0 "None" true 1.0 0.0 false
    (:then
      (Utilities|FlowControl|Sequence
        (:then_0
          (if (== (Utilities|Map|Length (Variables|Default|GetAttackMontageMap)) (Variables|Default|GetCurrentLgihtAttackComboCount))
            (CallFunction|ResetAttackComboCount)
            (else
              (Math|Integer|IncrementInt (Variables|Default|GetCurrentLgihtAttackComboCount)))))))
    (:OnCompleted
      (Ability|EndAbility :!label _label)
      (bind _returnvalue (Utilities|Time|SetTimerbyEvent (delegate Custom|ResetAttackComboCount) 1.0))
      (Variables|Default|SetComboCountResetTimerHandle _returnvalue))
    (:OnBlendOut
      (goto _label))
    (:OnInterrupted
      (goto _label))
    (:OnCancelled
      (goto _label))))

(event Ability|EventOnEndAbility
  (params (bWasCancelled :type Boolean)))