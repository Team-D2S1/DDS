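; Player heavy attack ability for the SGrip variant that chains combo montages from a map indexed by the combo count.
; On authority, a melee hit start event applies damage built from equipped weapon damage, attack type and combo count.
; The count advances after each montage starts, wraps after the last, and resets on a short timer once the montage ends.
; Activation requires a gameplay attribute comparison and a valid combo count.
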(event Custom|ResetAttackComboCount
  (Variables|Default|SetCurrentHeavyAttackComboCount 1))

(event Ability|EventActivateAbility
  (Utilities|Time|ClearandInvalidateTimerbyHandle (Variables|Default|GetComboCountResetTimerHandle))
  (|PlayMontageandWaitProxy "None" (.Value (Utilities|Map|Find (Variables|Default|GetAttackMontageMap) (Variables|Default|GetCurrentHeavyAttackComboCount))) 1.0 "None" true 1.0 0.0 false
    (:then
      (Ability|CommitAbility)
      (Utilities|FlowControl|Sequence
        (:then_0
          (Ability|HasAuthority
            (:True
              (bind _payload (Ability|Tasks|WaitGameplayEvent "(TagName=\"Shared.Event.MeleeHit.Start\")" 0)
                (:EventReceived
                  (Class|DDSGameplayAbility|ApplyEffectSpecHandletoTarget (.Target (Utilities|Struct|BreakGameplayEventData _payload)) (Class|DDSGameplayAbility|MakeGameplayEffectSpecHandle "/Game/Blueprints/Shared/GameplayEffect/GE_Shared_DealDamage.GE_Shared_DealDamage_C" (Class|PlayerCombatComponent|GetPlayerCurrentEquippedWeaponDamageatLevel (Class|DDSPlayerGameplayAbility|GetPlayerCombatComponentfromActorInfo) (Math|Conversions|ToFloat(Integer) (Ability|GetAbilityLevel))) "(TagName=\"Player.SetByCaller.AttackType.Heavy\")" (Variables|Default|GetCurrentHeavyAttackComboCount))))))))
        (:then_1
          (if (>= (Variables|Default|GetCurrentHeavyAttackComboCount) (Utilities|Map|Length (Variables|Default|GetAttackMontageMap)))
            (CallFunction|ResetAttackComboCount)
            (else
              (Math|Integer|IncrementInt (Variables|Default|GetCurrentHeavyAttackComboCount)))))))
    (:OnCompleted
      (Ability|EndAbility :!label _label)
      (bind _returnvalue (Utilities|Time|SetTimerbyEvent (delegate Custom|ResetAttackComboCount) 1.0))
      (Variables|Default|SetComboCountResetTimerHandle _returnvalue))
    (:OnBlendOut
      (goto _label))
    (:OnInterrupted
      (goto _label))
    (:OnCancelled
      (goto _label))))

(event Ability|EventOnEndAbility
  (params (bWasCancelled :type Boolean)))

(fn K2CanActivateAbility
  (params (ActorInfo :type Gameplay%20Ability%20Actor%20Info%20Structure) (Handle :type Gameplay%20Ability%20Spec%20Handle%20Structure))
  (bind _returnvalue (Ability|GetAbilitySystemComponentfromActorInfo))
  (return "" (and (>= (.ReturnValue (Class|AbilitySystemComponent|GetGameplayAttributeValue _returnvalue "(AttributeName=\"Stamina\",Attribute=/Script/DDS.DDSAttributeSet:Stamina,AttributeOwner=\"/Script/CoreUObject.Class'/Script/DDS.DDSAttributeSet'\")")) (.ReturnValue (Class|AbilitySystemComponent|GetGameplayAttributeValue _returnvalue "(AttributeName=\"AttackRequireStamina\",Attribute=/Script/DDS.DDSAttributeSet:AttackRequireStamina,AttributeOwner=\"/Script/CoreUObject.Class'/Script/DDS.DDSAttributeSet'\")"))) (>= (Utilities|Map|Length (Variables|Default|GetAttackMontageMap)) (Variables|Default|GetCurrentHeavyAttackComboCount)))))