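; Player light attack gameplay ability that plays a combo montage, advancing one step per activation.
; The montage comes from a map keyed by combo count, which wraps to the first step after the last.
; On authority, melee hit events apply a damage effect spec built from equipped weapon damage, attack type and executed combo count.
; Montage end or interruption ends the ability and starts a short combo reset timer, cleared on the next activation.
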(event Custom|ResetAttackComboCount
  (Variables|Default|SetCurrentLgihtAttackComboCount 1))

(event Ability|EventActivateAbility
  (Utilities|Time|ClearandInvalidateTimerbyHandle (Variables|Default|GetComboCountResetTimerHandle))
  (Variables|Default|SetExcutedComboCount (Variables|Default|GetCurrentLgihtAttackComboCount))
  (|PlayMontageandWaitProxy "None" (.Value (Utilities|Map|Find (Variables|Default|GetAttackMontageMap) (Variables|Default|GetCurrentLgihtAttackComboCount))) 1.0 "None" true 1.0 0.0 false
    (:then
      (Utilities|FlowControl|Sequence
        (:then_0
          (Ability|HasAuthority
            (:True
              (bind _payload (Ability|Tasks|WaitGameplayEvent "(TagName=\"Shared.Event.MeleeHit.Start\")" 0)
                (:EventReceived
                  (Class|DDSGameplayAbility|ApplyEffectSpecHandletoTarget (.Target (Utilities|Struct|BreakGameplayEventData _payload)) (Class|DDSGameplayAbility|MakeGameplayEffectSpecHandle 0 (Class|PlayerCombatComponent|GetPlayerCurrentEquippedWeaponDamageatLevel (Class|DDSPlayerGameplayAbility|GetPlayerCombatComponentfromActorInfo) (Math|Conversions|ToFloat(Integer) (Ability|GetAbilityLevel))) "(TagName=\"Player.SetByCaller.AttackType.Light\")" (Variables|Default|GetExcutedComboCount))))))))
        (:then_1
          (if (== (Utilities|Map|Length (Variables|Default|GetAttackMontageMap)) (Variables|Default|GetCurrentLgihtAttackComboCount))
            (CallFunction|ResetAttackComboCount)
            (else
              (Math|Integer|IncrementInt (Variables|Default|GetCurrentLgihtAttackComboCount)))))))
    (:OnCompleted
      (Ability|EndAbility :!label _label)
      (bind _returnvalue (Utilities|Time|SetTimerbyEvent (delegate Custom|ResetAttackComboCount) 1.0))
      (Variables|Default|SetComboCountResetTimerHandle _returnvalue))
    (:OnBlendOut
      (goto _label))
    (:OnInterrupted
      (goto _label))
    (:OnCancelled
      (goto _label))))

(event Ability|EventOnEndAbility
  (params (bWasCancelled :type Boolean)))