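; Player gameplay ability that unequips the sword with an unequip montage.
; On authority it clears the equipped weapon tag, then waits for a gameplay event to attach the sword to its side socket and call HandleUnequipWeapon.
; That function unlinks anim layers, removes granted weapon abilities and, if locally controlled, removes the input mapping context.
; Without authority, the ability only plays the montage and ends on its callbacks.
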(event Ability|EventActivateAbility
  (Ability|HasAuthority
    (:True
      (|PlayMontageandWaitProxy "None" "/Game/Blueprints/Player/Anim/Montages/AM_Warrior_Anim_UE_Unequip_Idle1.AM_Warrior_Anim_UE_Unequip_Idle1" 1.0 "None" true 1.0 0.0 false
        (:then
          (Variables|/Script/DDS.PawnCombatComponent|SetCurrentEquippedWeaponTag (Class|DDSPlayerGameplayAbility|GetPlayerCombatComponentfromActorInfo) "")
          (Ability|Tasks|WaitGameplayEvent "(TagName=\"Player.Event.Unequip.Sword\")" 0
            (:EventReceived
              (Transformation|AttachComponentToComponent (Class|PlayerCombatComponent|GetPlayerCarriedWeaponbyTag (Class|DDSPlayerGameplayAbility|GetPlayerCombatComponentfromActorInfo) "(TagName=\"Player.Weapon.Sword\")") (Class|GameplayAbility|GetOwningComponentfromActorInfo) "SwordSideSocket" "SnapToTarget" "KeepRelative" "KeepWorld" true)
              (CallFunction|HandleUnequipWeapon (Class|PlayerCombatComponent|GetPlayerCarriedWeaponbyTag (Class|DDSPlayerGameplayAbility|GetPlayerCombatComponentfromActorInfo) "(TagName=\"Player.Weapon.Sword\")")))))
        (:OnCompleted
          (Ability|EndAbility :!label _label))
        (:OnBlendedIn
          (goto _label))
        (:OnBlendOut
          (goto _label))
        (:OnInterrupted
          (goto _label))
        (:OnCancelled
          (goto _label))))
    (:False
      (Animation|Montage|PlayMontage (Class|GameplayAbility|GetOwningComponentfromActorInfo) "/Game/Blueprints/Player/Anim/Montages/AM_Warrior_Anim_UE_Unequip_Idle1.AM_Warrior_Anim_UE_Unequip_Idle1"
        (:OnCompleted
          _)
        (:OnBlendOut
          _)
        (:OnInterrupted
          _)
        (:OnNotifyBegin
          _)
        (:OnNotifyEnd
          _))
      (Ability|EndAbility))))

(event Ability|EventOnEndAbility
  (params (bWasCancelled :type Boolean)))

(fn HandleUnequipWeapon
  (params (InWeaponToUnequip :type DDS%20Player%20Weapon%20Object%20Reference))
  (LocalVariables|SetCachedPlayerWeaponData (Variables|/Script/DDS.DDSPlayerWeapon|GetPlayerWeaponData InWeaponToUnequip))
  (Ability|HasAuthority
    (:True
      (Utilities|FlowControl|Sequence
        (:then_0
          (Class|SkeletalMeshComponent|UnlinkAnimClassLayers (Class|GameplayAbility|GetOwningComponentfromActorInfo) (.WeaponAnimLayerToLink (Utilities|Struct|BreakDDSPlayerWeaponData (LocalVariables|GetCachedPlayerWeaponData)))))
        (:then_1
          (Pawn|IsLocallyControlled :!label _label
            (:True
              (Input|RemoveMappingContext (PlayerController|LocalPlayerSubsystems|GetEnhancedInputLocalPlayerSubsystem (Class|DDSPlayerGameplayAbility|GetPlayerControllerfromActorInfo)) (.WeaponInputMappingContext (Utilities|Struct|BreakDDSPlayerWeaponData (LocalVariables|GetCachedPlayerWeaponData))) "(bIgnoreAllPressedKeysUntilRelease=True,bForceImmediately=False,bNotifyUserSettings=False)"))))
        (:then_2
          (Class|DDSAbilitySystemComponent|RemoveGrantedPlayerWeaponAbilities (Class|DDSGameplayAbility|GetDDSAbilitySystemComponentfromActorInfo) (Class|DDSPlayerWeapon|GetGrantedAbilitySpecHandles InWeaponToUnequip)))))
    (:False
      (goto _label))))