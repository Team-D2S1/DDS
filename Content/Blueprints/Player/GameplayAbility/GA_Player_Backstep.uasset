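; GA_Player_Backstep is a player backstep gameplay ability, currently stubbed so that activation ends it immediately.
; Activation is gated on the avatar having a valid ability system component and a gameplay attribute at or above a fixed threshold.
; Disconnected logic plays a backward-jump montage, commits the ability, then ends it and applies a stamina-regen stop effect.
; Two placeholder-named helper functions remain, one empty and one choosing Front or Back.
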(event Ability|EventActivateAbility
  (Ability|EndAbility))

(event Ability|EventOnEndAbility
  (params (bWasCancelled :type Boolean)))

(fn NewFunction
  (params (Index :type Boolean)))

(fn NewFunction0
  (params (Index :type Boolean))
  (return (select Index "Front" "Back")))

(fn K2CanActivateAbility
  (params (ActorInfo :type Gameplay%20Ability%20Actor%20Info%20Structure) (Handle :type Gameplay%20Ability%20Spec%20Handle%20Structure))
  (bind _avataractor (Utilities|Struct|BreakGameplayAbilityActorInfo ActorInfo))
  (bind _returnvalue (Ability|GetAbilitySystemComponent _avataractor))
  (Utilities|IsValid _returnvalue
    (:Is%20Valid
      (return "" (>= (.ReturnValue (Class|AbilitySystemComponent|GetGameplayAttributeValue _returnvalue "(AttributeName=\"Stamina\",Attribute=/Script/DDS.DDSAttributeSet:Stamina,AttributeOwner=\"/Script/CoreUObject.Class'/Script/DDS.DDSAttributeSet'\")")) 1e+01)))))