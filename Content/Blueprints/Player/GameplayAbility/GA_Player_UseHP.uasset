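; Player gameplay ability that uses a health potion by applying the GE_HelthPotion effect to its owner.
; Activation applies the effect once and ends the ability immediately.
; The CanActivate override reads attributes from the owner's ability system component, requiring one to meet a small minimum and another to be below a third, likely potion charge and current versus maximum health.
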(event Ability|EventActivateAbility
  (Ability|ApplyGameplayEffectToOwner "/Game/Blueprints/Player/GameplayEffect/GE_HelthPotion.GE_HelthPotion_C")
  (Ability|EndAbility))

(event Ability|EventOnEndAbility
  (params (bWasCancelled :type Boolean)))

(fn K2CanActivateAbility
  (params (ActorInfo :type Gameplay%20Ability%20Actor%20Info%20Structure) (Handle :type Gameplay%20Ability%20Spec%20Handle%20Structure))
  (bind _returnvalue (Ability|GetAbilitySystemComponentfromActorInfo))
  (bind _returnvalue_2 (Class|AbilitySystemComponent|GetGameplayAttributeValue _returnvalue "(AttributeName=\"HealthPotion\",Attribute=/Script/DDS.DDSAttributeSet:HealthPotion,AttributeOwner=\"/Script/CoreUObject.Class'/Script/DDS.DDSAttributeSet'\")"))
  (return "" (and (>= _returnvalue_2 0.2) (< (.ReturnValue (Class|AbilitySystemComponent|GetGameplayAttributeValue _returnvalue "(AttributeName=\"Health\",Attribute=/Script/DDS.DDSAttributeSet:Health,AttributeOwner=\"/Script/CoreUObject.Class'/Script/DDS.DDSAttributeSet'\")")) (.ReturnValue (Class|AbilitySystemComponent|GetGameplayAttributeValue _returnvalue "(AttributeName=\"HealthMax\",Attribute=/Script/DDS.DDSAttributeSet:HealthMax,AttributeOwner=\"/Script/CoreUObject.Class'/Script/DDS.DDSAttributeSet'\")"))))))