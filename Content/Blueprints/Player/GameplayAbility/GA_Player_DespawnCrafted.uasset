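; Player gameplay ability that despawns the crafted weapon, first unequipping the current weapon through the combat component.
; The server unregisters the item by ID from the source ItemInstance or the weapon actor, destroys the actor, clears the equipped tag and ends.
; Clients only call the unequip, without ending the ability.
; A local HandleUnequipWeapon function, uncalled here, unlinks the anim layer and removes the input context and granted abilities.
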(event Ability|EventActivateAbility
  (bind _returnvalue (Class|DDSPlayerGameplayAbility|GetPlayerCombatComponentfromActorInfo))
  (bind _returnvalue_2 (Class|DDSPlayerGameplayAbility|GetPlayerCombatComponentfromActorInfo))
  (bind _returnvalue_3 (Class|DDSPlayerGameplayAbility|GetPlayerCombatComponentfromActorInfo))
  (Development|PrintString "Despawning")
  (Ability|HasAuthority
    (:True
      (Utilities|IsValid (Class|PlayerCombatComponent|GetPlayerCarriedWeaponbyTag _returnvalue (Variables|/Script/DDS.PawnCombatComponent|GetCurrentEquippedWeaponTag _returnvalue))
        (:Is%20Valid
          (Utilities|FlowControl|Sequence
            (:then_0
              (Class|PawnCombatComponent|HandleWeaponUnequip _returnvalue_2 (Class|PlayerCombatComponent|GetPlayerCarriedWeaponbyTag _returnvalue (Variables|/Script/DDS.PawnCombatComponent|GetCurrentEquippedWeaponTag _returnvalue))))
            (:then_1
              (Variables|Default|SetChachedActor (Class|PlayerCombatComponent|GetPlayerCarriedWeaponbyTag (Class|DDSPlayerGameplayAbility|GetPlayerCombatComponentfromActorInfo) "(TagName=\"Player.Weapon.Crafted\")") :!label _label)
              (bind _asitem_instance (Utilities|Casting|CastToItemInstance (Class|AbilitySystemBlueprintLibrary|EffectContextGetSourceObject))
                (:then
                  (Class|PawnCombatComponent|UnregisterSpawnedWeaponbyId _returnvalue_3 (Class|ItemInstance|GetItemId _asitem_instance)))
                (:CastFailed
                  (Class|PawnCombatComponent|UnregisterSpawnedWeaponbyId _returnvalue_3 (Class|DDSWeaponBase|GetItemId (Variables|Default|GetChachedActor)))))
              (Actor|DestroyActor (Variables|Default|GetChachedActor))
              (Variables|/Script/DDS.PawnCombatComponent|SetCurrentEquippedWeaponTag (Class|DDSPlayerGameplayAbility|GetPlayerCombatComponentfromActorInfo) "")
              (Ability|EndAbility))))
        (:Is%20Not%20Valid
          (goto _label))))
    (:False
      (Class|PawnCombatComponent|HandleWeaponUnequip _returnvalue_2 (Class|PlayerCombatComponent|GetPlayerCarriedWeaponbyTag _returnvalue (Variables|/Script/DDS.PawnCombatComponent|GetCurrentEquippedWeaponTag _returnvalue))))))

(event Ability|EventOnEndAbility
  (params (bWasCancelled :type Boolean)))

(fn HandleUnequipWeapon
  (params (InWeaponToUnequip :type DDS%20Crafted%20Player%20Weapon%20Object%20Reference))
  (LocalVariables|SetCachedPlayerWeaponData (Variables|/Script/DDS.DDSSimplePlayerWeapon|GetPlayerWeaponData InWeaponToUnequip))
  (Utilities|FlowControl|Sequence
    (:then_0
      (Ability|HasAuthority
        (:True
          (Class|EntityBase|MulticastUnlinkAnimLayer (Class|DDSPlayerGameplayAbility|GetPlayerCharacterfromActorInfo) (.WeaponAnimLayerToLink (Utilities|Struct|BreakDDSBaseWeaponData (LocalVariables|GetCachedPlayerWeaponData)))))))
    (:then_1
      (Pawn|IsLocallyControlled
        (:True
          (Input|RemoveMappingContext (PlayerController|LocalPlayerSubsystems|GetEnhancedInputLocalPlayerSubsystem (Class|DDSPlayerGameplayAbility|GetIngamePlayerControllerfromActorInfo)) (.WeaponInputMappingContext (Utilities|Struct|BreakDDSBaseWeaponData (LocalVariables|GetCachedPlayerWeaponData))) "(bIgnoreAllPressedKeysUntilRelease=True,bForceImmediately=False,bNotifyUserSettings=False)"))))
    (:then_2
      (Ability|HasAuthority
        (:True
          (Class|DDSAbilitySystemComponent|RemoveGrantedPlayerWeaponAbilities (Class|DDSGameplayAbility|GetDDSAbilitySystemComponentfromActorInfo) (Class|DDSSimplePlayerWeapon|GetGrantedAbilitySpecHandles InWeaponToUnequip)))))))