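; GA_Player_Evade is the player's evade gameplay ability, playing a directional dodge montage.
; It compares the axes of the normalized last dodge input from DDSAbilitySystemComponent to branch between two direction helpers.
; Only the Front/Back helper feeds montage selection; the Left/Right helper returns nothing, leaving side montages unreached.
; The ability commits after montage playback starts and ends on completion, blend-out, interruption or cancellation.
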(event Ability|EventActivateAbility
  (bind _asddsability_system_component (Utilities|Casting|CastToDDSAbilitySystemComponent (Ability|GetAbilitySystemComponentfromActorInfo)))
  (bind _output_get (Variables|Default|SetAs%20DDSAbility%20System%20Component _asddsability_system_component))
  (if (> (Math|Float|Absolute(Float) (.Y (Math|Vector|BreakVector (Math|Vector|Normalize (Class|DDSAbilitySystemComponent|GetLastDodgeInputDirection _output_get))))) (Math|Float|Absolute(Float) (.X (Math|Vector|BreakVector (Math|Vector|Normalize (Class|DDSAbilitySystemComponent|GetLastDodgeInputDirection _output_get))))))
    (CallFunction|NewFunction (>= (.X (Math|Vector|BreakVector (Math|Vector|Normalize (Class|DDSAbilitySystemComponent|GetLastDodgeInputDirection _output_get)))) 0.0))
    (else
      (bind _returnvalue (CallFunction|NewFunction0 (>= (.Y (Math|Vector|BreakVector (Math|Vector|Normalize (Class|DDSAbilitySystemComponent|GetLastDodgeInputDirection _output_get)))) 0.0)))))
  (|PlayMontageandWaitProxy "None" (Utilities|Select :Index _returnvalue :Left "/Game/Animations/Armot/AM_ARPG_Warrior_Anim_UE_Evade_Left_Montage.AM_ARPG_Warrior_Anim_UE_Evade_Left_Montage" :Right "/Game/Animations/Armot/AM_ARPG_Warrior_Anim_UE_Evade_Right_Montage.AM_ARPG_Warrior_Anim_UE_Evade_Right_Montage" :Up 0 :Down 0 :Front "/Game/Animations/Armot/AM_ARPG_Warrior_Anim_UE_Evade_Forward_Montage.AM_ARPG_Warrior_Anim_UE_Evade_Forward_Montage" :Back "/Game/Animations/Armot/AM_ARPG_Warrior_Anim_UE_Evade_Backward_Montage.AM_ARPG_Warrior_Anim_UE_Evade_Backward_Montage") 1.0 "None" true 1.0 0.0 false
    (:then
      (Ability|CommitAbility))
    (:OnCompleted
      (Ability|EndAbility :!label _label))
    (:OnBlendOut
      (goto _label))
    (:OnInterrupted
      (goto _label))
    (:OnCancelled
      (goto _label))))

(event Ability|EventOnEndAbility
  (params (bWasCancelled :type Boolean)))

(fn NewFunction
  (params (Index :type Boolean)))

(fn NewFunction0
  (params (Index :type Boolean))
  (return (select Index "Front" "Back")))